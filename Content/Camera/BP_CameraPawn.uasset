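; Camera pawn driven by speech recognition, turning the view in quarter or half turns and zooming in for a closer look or back out.
; Recognized phrases drive two timelines that lerp yaw, or pitch and field of view, with turns allowed only when zoomed out.
; Commands arriving mid-move can set queue flags, which Tick replays once movement stops.
; Repeated unknown phrases print a help message.
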(event Custom|OnWordsSpoken
  (params (Text :type Recognised%20Phrases%20Structure))
  (bind _camera (Variables|Default|GetCamera))
  (bind _camera_2 (Variables|Default|GetCamera))
  (bind _camera_3 (Variables|Default|GetCamera))
  (bind _relativerotation (Variables|/Script/Engine.SceneComponent|GetRelativeRotation _camera_2))
  (bind _relativerotation_2 (Variables|/Script/Engine.SceneComponent|GetRelativeRotation _camera_3))
  ;[0.08885 0.15 0.04847 0.5] Base Camera Movement
  (for _array_element (.phrases Text)
    (Development|PrintString _array_element)
    (switch string _array_element
      (:Turn%20Left
        (Variables|Default|SetRotationValue -9e+01)
        (if (Variables|Default|GetMoving) :!label _label
          (Variables|Default|SetQueueTurn (Variables|Default|GetZoomedIn))
          (elif (not (Variables|Default|GetZoomedIn))
            (bind _output_get (Variables|Default|SetRotationStart (.yaw _relativerotation_2)))
            (bind _output_get_2 (Variables|Default|SetRotationTarget (+ (.yaw _relativerotation_2) (Variables|Default|GetRotationValue))))
            (Variables|Default|SetMoving true)
            (Variables|Default|SetFailedCommands 0)
            (bind _newtrack_0 (Timeline|CameraRotation PlayFromStart)
              (:Update
                (Transformation|SetRelativeRotation (Variables|Default|GetCamera) (Math|Rotator|MakeRotator 0.0 0.0 (Math|Float|Lerp _output_get _output_get_2 _newtrack_0)) false false))
              (:Finished
                (Variables|Default|SetMoving false))))))
      (:Turn%20Right
        (Variables|Default|SetRotationValue 9e+01)
        (goto _label))
      (:Turn%20Around
        (Variables|Default|SetRotationValue 1.8e+02)
        (goto _label))
      (:Take%20a%20closer%20look
        (if (Variables|Default|GetMoving)
          (Variables|Default|SetQueueZoomIn true)
          (Variables|Default|SetFailedCommands 0 :!label _label_2)
          (elif (not (Variables|Default|GetZoomedIn))
            (Variables|Default|SetMoving true)
            (bind _newtrack_0_2 (Timeline|FocusZoom PlayFromStart)
              (:Update
                (Transformation|SetRelativeRotation _camera (Math|Rotator|MakeRotator (.roll _relativerotation) (Math|Float|Lerp 0.0 (Variables|Default|GetTargetTilt) _newtrack_0_2) (.yaw _relativerotation)) false false)
                (Camera|SetFieldOfView _camera (Math|Float|Lerp 9e+01 (Variables|Default|GetTargetFOV) _newtrack_0_2)))
              (:Finished
                (Variables|Default|SetMoving false)
                (Variables|Default|SetZoomedIn (not (Variables|Default|GetZoomedIn))))))))
      (:Step%20away
        (if (Variables|Default|GetMoving)
          (Variables|Default|SetQueueZoomOut true)
          (goto _label_2)
          (elif (Variables|Default|GetZoomedIn)
            (Variables|Default|SetMoving true)
            (Timeline|FocusZoom ReverseFromEnd)))))))

(event Custom|OnUnknownPhrase
  (bind _result (Math|Integer|IncrementInt (Variables|Default|GetFailedCommands))
    (:%20%20
      (if (>= _result 5)
        (Development|PrintString "Help message")
        (Variables|Default|SetFailedCommands 0)))))

(event EventBeginPlay
  (bind _returnvalue (Subsystems|GetSpeechRecognitionSubsystem))
  (EventDispatchers|BindEventtoOnWordsSpoken _returnvalue (delegate Custom|OnWordsSpoken))
  (EventDispatchers|BindEventtoOnUnknownPhrase _returnvalue (delegate Custom|OnUnknownPhrase)))

(event EventTick
  (params (DeltaSeconds :type Float%20%28single-precision%29))
  (bind _camera (Variables|Default|GetCamera))
  (bind _camera_2 (Variables|Default|GetCamera))
  (bind _camera_3 (Variables|Default|GetCamera))
  (bind _relativerotation (Variables|/Script/Engine.SceneComponent|GetRelativeRotation _camera_2))
  (bind _relativerotation_2 (Variables|/Script/Engine.SceneComponent|GetRelativeRotation _camera_3))
  ;[0.08885 0.15 0.04847 0.5] Base Camera Movement
  ;;[0.15 0.15 0.15 0.5] Command Queue
  (if (not (Variables|Default|GetMoving))
    (if (Variables|Default|GetQueueTurn)
      (Variables|Default|SetQueueTurn false)
      (if (Variables|Default|GetMoving)
        (Variables|Default|SetQueueTurn (Variables|Default|GetZoomedIn))
        (elif (not (Variables|Default|GetZoomedIn))
          (bind _output_get (Variables|Default|SetRotationStart (.yaw _relativerotation_2)))
          (bind _output_get_2 (Variables|Default|SetRotationTarget (+ (.yaw _relativerotation_2) (Variables|Default|GetRotationValue))))
          (Variables|Default|SetMoving true)
          (Variables|Default|SetFailedCommands 0)
          (bind _newtrack_0 (Timeline|CameraRotation PlayFromStart)
            (:Update
              (Transformation|SetRelativeRotation (Variables|Default|GetCamera) (Math|Rotator|MakeRotator 0.0 0.0 (Math|Float|Lerp _output_get _output_get_2 _newtrack_0)) false false))
            (:Finished
              (Variables|Default|SetMoving false)))))
      (elif (Variables|Default|GetZoomedIn)
        (if (Variables|Default|GetQueueZoomOut)
          (Variables|Default|SetQueueZoomOut false)
          (Variables|Default|SetMoving true)
          (bind _newtrack_0_2 (Timeline|FocusZoom ReverseFromEnd)
            (:Update
              (Transformation|SetRelativeRotation _camera (Math|Rotator|MakeRotator (.roll _relativerotation) (Math|Float|Lerp 0.0 (Variables|Default|GetTargetTilt) _newtrack_0_2) (.yaw _relativerotation)) false false)
              (Camera|SetFieldOfView _camera (Math|Float|Lerp 9e+01 (Variables|Default|GetTargetFOV) _newtrack_0_2)))
            (:Finished
              (Variables|Default|SetMoving false)
              (Variables|Default|SetZoomedIn (not (Variables|Default|GetZoomedIn))))))
        (elif (Variables|Default|GetQueueZoomIn)
          (Variables|Default|SetQueueZoomIn false)
          (Variables|Default|SetMoving true)
          (Timeline|FocusZoom PlayFromStart))))))

(fn ConstructionScript)